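; BP_TankCharacter is a tank character Blueprint with a debug mode that simulates back-and-forth movement.
; The X debug key toggles the simulation and resets its direction timer.
; While active, Tick feeds movement input along the world X axis and flips its sign whenever the timer exceeds TimeToMoveForward.
; The SimulateCharacterMove function is an empty stub with a disconnected direction toggle.
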(event EventBeginPlay)

(event Collision|EventActorBeginOverlap
  (params (OtherActor :type Actor%20Object%20Reference)))

(event EventTick
  (params (DeltaSeconds :type Float%20%28single-precision%29))
  (if (Variables|Default|GetSimulateCharacterMovement)
    (Pawn|Input|AddMovementInput "1.000000,0.000000,0.000000" (Math|Float|SelectFloat 1.0 -1.0 (Variables|Default|GetMovingForward)) false)
    (Variables|Default|SetTimeSinceDirectionChange (+ (Variables|Default|GetTimeSinceDirectionChange) DeltaSeconds))
    (if (> (Variables|Default|GetTimeSinceDirectionChange) (Variables|Default|GetTimeToMoveForward))
      (Variables|Default|SetTimeSinceDirectionChange 0.0)
      (Variables|Default|SetMovingForward (not (Variables|Default|GetMovingForward))))))

(event Input|KeyboardEvents|DebugKeyX
  (params (Key :type Key%20Structure :default "None") (ActionValue :type Input%20Action%20Value%20Structure))
  (:Pressed
    (Variables|Default|SetSimulateCharacterMovement (not (Variables|Default|GetSimulateCharacterMovement)))
    (Variables|Default|SetTimeSinceDirectionChange 0.0)))

(fn ConstructionScript)

(fn SimulateCharacterMove
  (params (InputPin :type Float%20%28single-precision%29)))